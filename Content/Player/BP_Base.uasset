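; BP_Base is a base character Blueprint that provides shared health, action state and movement-mode logic.
; An enum StateType, with a setter and a query per state, tracks idle, roll, backstep, equip, action, down and dead states.
; Health adjustment clamps the value and reports survival, and helpers toggle between flying and walking.
; Weapon and behavior-end functions and the SkillData event are empty stubs, apparently meant for child overrides.
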(event `SkillData`
  (params (Amount :type "Float (double-precision)") (StartPoint :type "Vector Structure") (EndPoint :type "Vector Structure") (TargetCount :type Integer) (bDoing :type Boolean) (Amount2 :type "Float (double-precision)")))

(fn `Adjust Health`
  (params (InDamage :type "Float (double-precision)"))
  (returns (Return :type Boolean))
  (bind _output_get (set `self.Health` (`KismetMathLibrary.FClamp` (- (`self.Health`) InDamage) 0.0 (`self.MaxHealth`))))
  (if (> _output_get 0.0)
    (return true)
    (else
      (return false))))

(fn `Behavior_EndBackStep`
  (returns (Result :type Boolean))
  (return false))

(fn `Behavior_EndDead`
  (returns (Result :type Boolean))
  (return false))

(fn `Behavior_EndHitted`
  (returns (Result :type Boolean))
  (return false))

(fn `Behavior_EndRoll`
  (returns (Result :type Boolean))
  (return false))

(fn `Behavior_EndTumbling`
  (returns (Result :type Boolean))
  (return false))

(fn `EndDead`
  (set `self.StateType` "NewEnumerator6"))

(fn `EndFlyingMode`
  (`CharacterMovementComponent.SetMovementMode` (`self.CharacterMovement`) "MOVE_Walking" 0)
  (return))

(fn `GetWeapon_Current`
  (returns (OutWeapon :type "/Game/Weapon/BP_Weapon Object Reference"))
  (return null))

(fn `IsState_Action`
  (returns (Result :type Boolean))
  (return (`|EnumEquality` (`self.StateType`) "NewEnumerator4")))

(fn `IsState_AirDown`
  (returns (Result :type Boolean))
  (return (`|EnumEquality` (`self.StateType`) "NewEnumerator8")))

(fn `IsState_Backup`
  (returns (Result :type Boolean))
  (return (`|EnumEquality` (`self.StateType`) "NewEnumerator2")))

(fn `IsState_Dead`
  (returns (Result :type Boolean))
  (return (`|EnumEquality` (`self.StateType`) "NewEnumerator6")))

(fn `IsState_Down`
  (returns (Result :type Boolean))
  (return (`|EnumEquality` (`self.StateType`) "NewEnumerator9")))

(fn `IsState_Equip`
  (returns (Result :type Boolean))
  (return (`|EnumEquality` (`self.StateType`) "NewEnumerator3")))

(fn `IsState_Idle`
  (returns (Result :type Boolean))
  (return (`|EnumEquality` (`self.StateType`) "NewEnumerator0")))

(fn `IsState_Roll`
  (returns (Result :type Boolean))
  (return (`|EnumEquality` (`self.StateType`) "NewEnumerator1")))

(fn `SetFlyingMode`
  (`CharacterMovementComponent.SetMovementMode` (`self.CharacterMovement`) "MOVE_Flying" 0)
  (return))

(fn `SetState_Action`
  (returns (Result :type Boolean))
  (set `self.StateType` "NewEnumerator4")
  (return false))

(fn `SetState_AirDown`
  (returns (Result :type Boolean))
  (set `self.StateType` "NewEnumerator8")
  (return false))

(fn `SetState_Backup`
  (returns (Result :type Boolean))
  (set `self.StateType` "NewEnumerator2")
  (return false))

(fn `SetState_Dead`
  (returns (Result :type Boolean))
  (set `self.StateType` "NewEnumerator6")
  (return false))

(fn `SetState_Down`
  (returns (Result :type Boolean))
  (set `self.StateType` "NewEnumerator9")
  (return false))

(fn `SetState_Equip`
  (returns (Result :type Boolean))
  (set `self.StateType` "NewEnumerator3")
  (return false))

(fn `SetState_Idle`
  (returns (Result :type Boolean))
  (set `self.StateType` "NewEnumerator0")
  (return false))

(fn `SetState_Roll`
  (returns (Result :type Boolean))
  (set `self.StateType` "NewEnumerator1")
  (return false))

(fn `UserConstructionScript`)

(fn `Weapon_Begin_Equip`
  (returns (Result :type Boolean))
  (return false))

(fn `Weapon_Change`
  (params (InWeapon :type "/Game/Weapon/BP_Weapon Object Reference"))
  (returns (Result :type Boolean))
  (return false))

(fn `Weapon_End_Equip`
  (returns (Result :type Boolean))
  (return false))

(fn `Weapon_Move`
  (returns (Result :type Boolean))
  (return false))

(fn `Weapon_Stop`
  (returns (Result :type Boolean))
  (return false))