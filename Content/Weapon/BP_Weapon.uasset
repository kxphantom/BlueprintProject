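; Base weapon actor that gives its owning character equip state, socket attachment, montage attacks and damage.
; On BeginPlay it loads every ActionTable row into ActionDatas and caches the owner Character; getters filter rows by WeaponType for damage, effect, camera shake, sound and stop data.
; PlayAction plays the indexed montage and tells the owner whether it can move.
; BeginEquip and the DoAction functions are empty stubs, while SendDamage excludes owner and self.
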(event `self.ReceiveBeginPlay`
  (`|ExecutionSequence`
    (:`then_0`
      (bind _actiontable (`self.ActionTable`)
        (:`then`
          (bind _outrownames (`DataTableFunctionLibrary.GetDataTableRowNames` _actiontable))
          (for _array_element _outrownames
            (bind _returnvalue (`|GetDataTableRow` (`self.ActionTable`) _array_element)
              (:`then`
                (`KismetArrayLibrary.Array_Add` (`self.ActionDatas`) _returnvalue)))))
        (:`else`)))
    (:`then_1`
      (bind _ascharacter (cast `Character` (`self.GetOwner`)))
      (set `self.OwnerCharacter` _ascharacter))))

(fn `AttachToOwnerCharacter`
  (params (InSocketName :type Name))
  (`self.K2_AttachToComponent` (`Character.Mesh` (`self.OwnerCharacter`)) InSocketName "KeepRelative" "KeepRelative" "KeepRelative"))

(fn `Begin_DoAction`)

(fn `Begin_Equip`)

(fn `Do Action`)

(fn `End_DoAction`)

(fn `End_Equip`
  (set `self.Equipped` true))

(fn `GetActionCamera`
  (params (InIndex :type Integer))
  (returns (`Camera Shake` :type "MatineeCameraShake Class Reference"))
  (bind (_output_type _output_montage _output_playratio _output_startsectionname _output_canmove _output_attack _output_stop _output_effect _output_effectlocation _output_effectscale _output_effectrotation _output_camerashake) (break `/Game/Structures/FAction` (`|GetArrayItem` (`self.GetActions`) InIndex)))
  (return _output_camerashake))

(fn `GetActionDamage`
  (params (InIndex :type Integer))
  (returns (Attack :type "Float (double-precision)"))
  (bind (_output_type _output_montage _output_playratio _output_startsectionname _output_canmove _output_attack) (break `/Game/Structures/FAction` (`|GetArrayItem` (`self.GetActions`) InIndex)))
  (return _output_attack))

(fn `GetActionData`
  (params (InIndex :type Integer))
  (returns (Result :type "/Game/Structures/FAction Structure"))
  (bind _actiondatas (`self.ActionDatas`))
  (if (< InIndex (`KismetArrayLibrary.Array_Length` _actiondatas))
    (return (`|GetArrayItem` _actiondatas (`local.InIndex`)))))

(fn `GetActionEffect`
  (params (InIndex :type Integer))
  (returns (Effect :type "ParticleSystem Object Reference") (`Effect Location` :type "Vector Structure") (`Effect Scale` :type "Vector Structure") (`Effect Rotation` :type "Rotator Structure"))
  (bind (_output_type _output_montage _output_playratio _output_startsectionname _output_canmove _output_attack _output_stop _output_effect _output_effectlocation _output_effectscale _output_effectrotation) (break `/Game/Structures/FAction` (`|GetArrayItem` (`self.GetActions`) InIndex)))
  (return _output_effect _output_effectlocation _output_effectscale _output_effectrotation))

(fn `GetActions`
  (returns (OutActions :type "Array of /Game/Structures/FAction Structure"))
  (locals (Actions :type "Array of /Game/Structures/FAction Structure"))
  (for _array_element (`self.ActionDatas`)
    (if (`|EnumEquality` (`.Type_7_E4CDAF5E4D578A7ACDD782AEC0300A83` (break `/Game/Structures/FAction` _array_element)) (`self.WeaponType`))
      (`KismetArrayLibrary.Array_Add` (`local.Actions`) _array_element)))
  (return (`local.Actions`)))

(fn `GetActionSound`
  (params (InIndex :type Integer))
  (returns (`Sound Cue` :type "SoundCue Object Reference"))
  (bind (_output_type _output_montage _output_playratio _output_startsectionname _output_canmove _output_attack _output_stop _output_effect _output_effectlocation _output_effectscale _output_effectrotation _output_camerashake _output_soundcue) (break `/Game/Structures/FAction` (`|GetArrayItem` (`self.GetActions`) InIndex)))
  (return _output_soundcue))

(fn `GetActionStop`
  (params (InIndex :type Integer))
  (returns (Stop :type "Float (double-precision)"))
  (bind (_output_type _output_montage _output_playratio _output_startsectionname _output_canmove _output_attack _output_stop) (break `/Game/Structures/FAction` (`|GetArrayItem` (`self.GetActions`) InIndex)))
  (return _output_stop))

(fn `GetEquipped`
  (returns (Equipped :type Boolean))
  (return (`self.Equipped`)))

(fn `IsExistAction`
  (returns (OutResult :type Boolean))
  (for _array_element (`self.ActionDatas`)
    (if (`|EnumEquality` (break `/Game/Structures/FAction` _array_element) (`self.WeaponType`))
      (return true)))
  (return false))

(fn `PlayAction`
  (params (InIndex :type Integer))
  (bind _ownercharacter (`self.OwnerCharacter`))
  (bind (_output_type _output_montage _output_playratio _output_startsectionname _output_canmove) (break `/Game/Structures/FAction` (`|GetArrayItem` (`self.GetActions`) InIndex)))
  (`Character.PlayAnimMontage` (`self.OwnerCharacter`) _output_montage _output_playratio _output_startsectionname)
  (if _output_canmove
    (message `/Game/Interfaces/IWeapon.Weapon_Move` _ownercharacter)
    (else
      (message `/Game/Interfaces/IWeapon.Weapon_Stop` _ownercharacter))))

(fn `SendDamage`
  (params (InOtherActor :type "Actor Object Reference") (InDamage :type "Float (double-precision)"))
  (if (and (!= InOtherActor (`self.OwnerCharacter`)) (!= InOtherActor self))
    (`GameplayStatics.ApplyDamage` (`local.InOtherActor`) (`local.InDamage`) (`Pawn.GetController` (`self.OwnerCharacter`)) self)))

(fn `Unequip`
  (set `self.Equipped` false))

(fn `UserConstructionScript`)