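; Melee weapon Blueprint that extends a parent weapon with a combo attack chain, driven through the owner's IState and IWeapon interfaces.
; Input during the combo window queues the next indexed action, which BeginDoAction plays; EndDoAction resets the chain and owner state.
; All shape components share an overlap handler and collision toggles, while SendDamage records hit actors to damage each once until collision switches off.
; A helper restores global time dilation.
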(event `self.ReceiveBeginPlay`
  (`parent.ReceiveBeginPlay`)
  (`self.RegistBeginOverlap`)
  (`self.OffCollision`))

(event `self.Do Action`
  (bind _ownercharacter (`self.OwnerCharacter`))
  ;[1 1 1] DoAction
  (`parent.Do Action`)
  (if (`self.IsExistAction`)
    (if (`self.Enable`)
      (set `self.Enable` false)
      (set `self.Exist` true)
      (elif (`KismetSystemLibrary.DoesImplementInterface` _ownercharacter "/Game/Interfaces/IState.IState_C")
        (bind _result (message `/Game/Interfaces/IState.IsState_Idle` _ownercharacter))
        (if _result
          (message `/Game/Interfaces/IState.SetState_Action` _ownercharacter)
          (`self.PlayAction` (`self.Index`)))))))

(event `self.Begin_DoAction`
  (bind _index (`self.Index`))
  ;[1 1 1] Begin Do Action
  (`parent.Begin_DoAction`)
  (if (`self.Exist`)
    (set `self.Exist` false)
    (`Character.StopAnimMontage` (`self.OwnerCharacter`) null)
    (`/Engine/EditorBlueprintResources/StandardMacros.IncrementInt` _index
      (:`  `
        (`self.PlayAction` _index)))))

(event `self.End_DoAction`
  (bind _ownercharacter (`self.OwnerCharacter`))
  (bind _ownercharacter_2 (`self.OwnerCharacter`))
  ;[1 1 1] End Do Action
  (`parent.End_DoAction`)
  (`Character.StopAnimMontage` (`self.OwnerCharacter`) null)
  (set `self.Index` 0)
  (if (`KismetSystemLibrary.DoesImplementInterface` _ownercharacter_2 "/Game/Interfaces/IState.IState_C")
    (message `/Game/Interfaces/IState.SetState_Idle` _ownercharacter_2)
    (if (`KismetSystemLibrary.DoesImplementInterface` _ownercharacter "/Game/Interfaces/IWeapon.IWeapon_C")
      (message `/Game/Interfaces/IWeapon.Weapon_Move` _ownercharacter))))

(event `End_EnableCombo`
  ;[1 1 1] Enable Combo
  (set `self.Enable` false))

(event `Begin_EnableCombo`
  ;[1 1 1] Enable Combo
  (set `self.Enable` true))

(event `self.SendDamage`
  (params (InOtherActor :type "Actor Object Reference") (InDamage :type "Float (single-precision)"))
  ;[1 1 1] Send Damage
  (if (< (`KismetArrayLibrary.Array_Find` (`self.Hitted Actors`) InOtherActor) 0)
    (`KismetArrayLibrary.Array_Add` (`self.Hitted Actors`) InOtherActor)
    (`parent.SendDamage` InOtherActor InDamage)))

(fn `Begin_Equip`
  (`parent.Begin_Equip`))

(fn `OffCollision`
  (for _array_element (`self.K2_GetComponentsByClass` "/Script/Engine.ShapeComponent")
    (`PrimitiveComponent.SetCollisionEnabled` _array_element "NoCollision")
    (`KismetArrayLibrary.Array_Clear` (`self.Hitted Actors`))))

(fn `OnBeginOverlap`
  (params (OverlappedComponent :type "PrimitiveComponent Object Reference") (OtherActor :type "Actor Object Reference") (OtherComp :type "PrimitiveComponent Object Reference") (OtherBodyIndex :type Integer) (bFromSweep :type Boolean) (SweepResult :type "HitResult Structure (by ref)"))
  (if (and (!= OtherActor (`self.OwnerCharacter`)) (!= OtherActor self))
    (`|ExecutionSequence`)))

(fn `OnCollision`
  (for _array_element (`self.K2_GetComponentsByClass` "/Script/Engine.ShapeComponent")
    (`PrimitiveComponent.SetCollisionEnabled` _array_element "QueryAndPhysics")))

(fn `RegistBeginOverlap`
  (for _array_element (`self.K2_GetComponentsByClass` "/Script/Engine.ShapeComponent")
    (add `PrimitiveComponent.OnComponentBeginOverlap` _array_element (`|CreateDelegate` :!event `OnBeginOverlap`))))

(fn `RestoreStopTimer`
  (`GameplayStatics.SetGlobalTimeDilation` 1.0))

(fn `Unequip`
  (`parent.Unequip`))

(fn `UserConstructionScript`
  (`parent.UserConstructionScript`))