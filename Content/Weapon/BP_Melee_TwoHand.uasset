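; Two-handed melee weapon Blueprint (a void sword) that extends a parent weapon class with socket attachment and a ribbon trail effect.
; It attaches to the owner's holster on spawn and unequip, and to the hand when equipping.
; Actions switch the Niagara trail on and off, setting its ribbon width.
; Tick hides the sword mesh while the player dashes and feeds the mesh's world rotation into Niagara's relative rotation.
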(event `self.ReceiveBeginPlay`
  (`parent.ReceiveBeginPlay`)
  (`self.AttachToOwnerCharacter` "Holster_TwoHand"))

(event `self.Begin_Equip`
  (`parent.Begin_Equip`)
  (`self.AttachToOwnerCharacter` "Hand_TwoHand"))

(event `self.Unequip`
  (`parent.Unequip`)
  (`self.AttachToOwnerCharacter` "Holster_TwoHand"))

(event `self.Do Action`
  (`parent.Do Action`)
  (`ActorComponent.Activate` (`self.Niagara`) false)
  (`NiagaraComponent.SetVariableFloat` (`self.Niagara`) "User.RibbonWidth" 200.0))

(event `self.End_DoAction`
  (`parent.End_DoAction`)
  (`ActorComponent.Deactivate` (`self.Niagara`)))

(event `self.ReceiveTick`
  (params (DeltaSeconds :type "Float (single-precision)"))
  (bind _sm_void_sword_sword (`self.SM_Void_Sword_Sword`))
  ;[1 1 1] Tick
  (`|ExecutionSequence`
    (:`then_0`
      (bind _asbp_player (cast `/Game/Player/BP_Player` (`self.OwnerCharacter`))) ; 대쉬 확인
      (bind _dashing (`/Game/Player/BP_Player.IsDashing` _asbp_player))
      (if _dashing
        (`SceneComponent.SetVisibility` _sm_void_sword_sword false false)
        (else
          (`SceneComponent.SetVisibility` _sm_void_sword_sword true false))))
    (:`then_1`
      (`SceneComponent.K2_SetRelativeRotation` (`self.Niagara`) (`SceneComponent.K2_GetComponentRotation` (`self.SM_Void_Sword_Sword`)) false false))))

(fn `UserConstructionScript`
  (`parent.UserConstructionScript`))