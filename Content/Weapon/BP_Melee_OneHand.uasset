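; One-handed melee weapon that extends a parent weapon Blueprint, moving between a holster socket and a hand socket on equip and unequip.
; On BeginPlay it attaches each of its sphere components to the owner's mesh socket of the same name.
; Each action activates Niagara effects chosen by index, and ending the action deactivates them all.
; Tick hides the weapon mesh while a player owner dashes and shows it again when idle.
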(event `self.ReceiveBeginPlay`
  ;[1 1 1] BeginPlay
  (`parent.ReceiveBeginPlay`)
  (`self.AttachToOwnerCharacter` "Holster_OneHand")
  (for _array_element (`self.K2_GetComponentsByClass` "/Script/Engine.SphereComponent")
    (`SceneComponent.K2_AttachToComponent` _array_element (`Character.Mesh` (`self.OwnerCharacter`)) (`KismetStringLibrary.Conv_StringToName` (`KismetSystemLibrary.GetObjectName` _array_element)) "KeepRelative" "KeepRelative" "KeepRelative" true)))

(event `self.Begin_Equip`
  ;[1 1 1] Equip
  (`parent.Begin_Equip`)
  (`self.AttachToOwnerCharacter` "Hand_OneHand")
  (`SceneComponent.SetVisibility` (`self.OneHand`) true false))

(event `self.Unequip`
  ;[1 1 1] Equip
  (`parent.Unequip`)
  (`self.AttachToOwnerCharacter` "Holster_OneHand")
  (`SceneComponent.SetVisibility` (`self.OneHand`) false false))

(event `self.Do Action`
  ;[1 1 1] DoAction
  (`parent.Do Action`)
  (switch `int` (`self.Index`)
    (:`0`
      (`ActorComponent.Activate` (`self.Niagara`) false :!label _label))
    (:`1`
      (`ActorComponent.Activate` (`self.Niagara1`) false :!label _label_2)
      (`ActorComponent.Activate` (`self.Niagara2`) false))
    (:`2`
      (goto _label_2))
    (:`3`
      (goto _label))))

(event `self.End_DoAction`
  ;[1 1 1] End DoAction
  (`parent.End_DoAction`)
  (`ActorComponent.Deactivate` (`self.Niagara`))
  (`ActorComponent.Deactivate` (`self.Niagara1`))
  (`ActorComponent.Deactivate` (`self.Niagara2`)))

(event `self.ReceiveTick`
  (params (DeltaSeconds :type "Float (single-precision)"))
  (bind _asbp_player (cast `/Game/Player/BP_Player` (`self.OwnerCharacter`)))
  (bind _dashing (`/Game/Player/BP_Player.IsDashing` _asbp_player))
  (if _dashing
    (`SceneComponent.SetVisibility` (`self.OneHand`) false false)
    (else
      (bind _result (message `/Game/Interfaces/IState.IsState_Idle` (`self.OwnerCharacter`)))
      (if _result
        (`SceneComponent.SetVisibility` (`self.OneHand`) true false)))))

(fn `UserConstructionScript`
  (`parent.UserConstructionScript`))